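; Steampunk balloon prop that assembles its rigging procedurally and animates a pulsing, swaying point light.
; The construction script rings top ropes and side chains around the center as evenly rotated hierarchical instanced static meshes.
; Each tick, a clamped sine-of-real-time waveform scales the light up to LightIntensity.
; The same normalized value shifts the light in X and Y around its position cached at BeginPlay.
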(event EventBeginPlay
  (Variables|Default|SetOriginalLightLocation (Variables|/Script/Engine.SceneComponent|GetRelativeLocation (Variables|Default|GetPointLight))))

(event Collision|EventActorBeginOverlap
  (params (OtherActor :type Actor%20Object%20Reference)))

(event EventTick
  (params (DeltaSeconds :type Float%20%28single-precision%29))
  (bind _returnvalue (Utilities|Time|GetRealTimeSeconds))
  (bind _lightintensity (Variables|Default|GetLightIntensity))
  (bind _originallightlocation (Variables|Default|GetOriginalLightLocation))
  (bind _pointlight (Variables|Default|GetPointLight))
  (bind _returnvalue_2 (Math|Trig|Sin(Radians) _returnvalue))
  (bind _returnvalue_3 (/ _returnvalue_2 4.0))
  (bind _returnvalue_4 (Math|Float|Absolute(Float) _returnvalue_2))
  (bind _returnvalue_5 (/ _returnvalue_4 2.0))
  (bind _returnvalue_6 (+ _returnvalue_3 0.5))
  (bind _returnvalue_7 (+ _returnvalue_6 _returnvalue_5))
  (bind _returnvalue_8 (* _lightintensity _returnvalue_7))
  (bind _returnvalue_9 (Math|Float|Clamp(Float) _returnvalue_8 0.0 _lightintensity))
  (bind _returnvalue_10 (/ _returnvalue_9 _lightintensity))
  (bind _returnvalue_11 (- _returnvalue_10 0.5))
  (Rendering|Components|Light|SetIntensity _pointlight _returnvalue_9)
  (Transformation|SetRelativeLocation _pointlight (Math|Vector|MakeVector (+ (* _returnvalue_11 2.0) (.x _originallightlocation)) (+ (* _returnvalue_11 5.0) (.y _originallightlocation)) (.z _originallightlocation)) false false))

(fn ConstructionScript
  (Utilities|FlowControl|Sequence
    (:then_0
      (for _index (range 0 9)
        (Components|InstancedStaticMesh|AddInstance (Variables|Default|GetHISM_topropes) (Math|Transform|MakeTransform "0, 0, 0" (Math|Rotator|MakeRotator 0.0 0.0 (* _index 36.0))))))
    (:then_1
      (for _index_2 (range 0 3)
        (Components|InstancedStaticMesh|AddInstance (Variables|Default|GetHISM_sidechain) (Math|Transform|MakeTransform "0, 0, 0" (Math|Rotator|MakeRotator 0.0 0.0 (* _index_2 9e+01))))))))